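; AI guard for the shooter that takes damage and shows its health on a widget-based health bar.
; On BeginPlay, the guard type (Normal or Heavy) sets max health, and the widget is cached as a UI_ProgressBar.
; Damage is converted to a fraction of max health and sent to the red bar.
; The guard stores no current health, so the bar update's return value decides when it is destroyed.
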(event `self.ReceiveBeginPlay`
  ;[1 1 1] Set Guard Type, Health And Display Health Bar
  (switch `/Game/Shooter/Enums/E_GuardType` (`self.GuardType`)
    (:`NewEnumerator0`
      (set `self.MaxHealth` 100))
    (:`NewEnumerator1`
      (set `self.MaxHealth` 200)))
  (bind _asui_progress_bar (cast `/Game/Shooter/UI/UI_ProgressBar` (`WidgetComponent.GetWidget` (`self.HealthBarWidget`))))
  (set `self.HealthBar` _asui_progress_bar))

(event `/Game/Shooter/Blueprints/BPI_Guard.TakeDamage`
  (params (Damage :type "Float (double-precision)"))
  ;[1 1 1] Guard Taking Damage
  (bind _isvalid (`/Game/Shooter/UI/UI_ProgressBar.UpdateProgressBar` (`self.HealthBar`) (struct :`R` 1.0 :`A` 1.0) (`KismetMathLibrary.MapRangeClamped` Damage 0.0 (`KismetMathLibrary.Conv_IntToDouble` (`self.MaxHealth`)) 0.0 1.0)))
  (if (not _isvalid)
    (`self.K2_DestroyActor`)))

(fn `UserConstructionScript`)