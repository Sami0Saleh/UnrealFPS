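; Shootable weapon Blueprint that fires physics-driven bullets as a rifle or machinegun, depending on its current weapon type.
; Attack, ignored while hidden, waits a type-specific delay, spawns a BP_Bullet at the barrel pivot, passes it the type and launches it by impulse.
; Each shot uses ammo and refreshes the HUD through PC_New, while an empty weapon prints a message.
; AddAmmo refills ammo, capped at magazine size.
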(event `/Game/Shooter/Blueprints/BPI_Weapon.WeaponType`
  (params (NewParam :type "/Game/Shooter/Enums/E_WeaponType Enum" :default "NewEnumerator3"))
  ;[1 1 1] Set  Weapon Type
  (set `self.CurrentWeaponType` NewParam))

(event `/Game/Shooter/Blueprints/BPI_Weapon.Attack`
  ;[1 1 1] Shooting The Weapon
  (if (not (`self.bHidden`))
    (switch `/Game/Shooter/Enums/E_WeaponType` (`self.CurrentWeaponType`)
      (:`NewEnumerator0`
        (if (> (`self.AmmoAmount`) 0)
          (`KismetSystemLibrary.Delay` 0.5)
          (bind _returnvalue (`|SpawnActorFromClass` "/Game/Shooter/Blueprints/BP_Bullet.BP_Bullet_C" (`KismetMathLibrary.MakeTransform` (`SceneComponent.K2_GetComponentLocation` (`self.BarrelPivot`)) (struct) (0.05 0.05 0.05)) "AlwaysSpawn" "MultiplyWithRoot" null null))
          (message `/Game/Shooter/Blueprints/BPI_Bullet.Get WeaponType` _returnvalue (`self.CurrentWeaponType`))
          (`PrimitiveComponent.AddImpulse` (`/Game/Shooter/Blueprints/BP_Bullet.Sphere` _returnvalue) (* (`SceneComponent.GetForwardVector` (`self.BarrelPivot`)) 500.0) "None" false)
          (`/Engine/EditorBlueprintResources/StandardMacros.DecrementInt` (`self.AmmoAmount`)
            (:`  `
              (bind _returnvalue_2 (`GameplayStatics.GetActorOfClass` "/Game/Shooter/Blueprints/PC_New.PC_New_C"))
              (`/Game/Shooter/Blueprints/PC_New.UpdateHUD` _returnvalue_2)))
          (else
            (`KismetSystemLibrary.PrintString` "No bullets!"))))
      (:`NewEnumerator1`
        (if (> (`self.AmmoAmount`) 0)
          (`KismetSystemLibrary.Delay` 0.2)
          (bind _returnvalue_3 (`|SpawnActorFromClass` "/Game/Shooter/Blueprints/BP_Bullet.BP_Bullet_C" (`KismetMathLibrary.MakeTransform` (`SceneComponent.K2_GetComponentLocation` (`self.BarrelPivot`)) (struct) (0.05 0.05 0.05)) "AlwaysSpawn" "MultiplyWithRoot" null null))
          (message `/Game/Shooter/Blueprints/BPI_Bullet.Get WeaponType` _returnvalue_3 (`self.CurrentWeaponType`))
          (`PrimitiveComponent.AddImpulse` (`/Game/Shooter/Blueprints/BP_Bullet.Sphere` _returnvalue_3) (* (`SceneComponent.GetForwardVector` (`self.BarrelPivot`)) 1000.0) "None" false)
          (`/Engine/EditorBlueprintResources/StandardMacros.DecrementInt` (`self.AmmoAmount`)
            (:`  `
              (bind _returnvalue_4 (`GameplayStatics.GetActorOfClass` "/Game/Shooter/Blueprints/PC_New.PC_New_C"))
              (`/Game/Shooter/Blueprints/PC_New.UpdateHUD` _returnvalue_4)))
          (else
            (`KismetSystemLibrary.PrintString` "No bullets!")))))))

(event `/Game/Shooter/Blueprints/BPI_Weapon.AddAmmo`
  (params (Ammo :type Integer))
  ;[1 1 1] Add Ammo To Weapon
  (bind _output_get (set `self.AmmoAmount` (+ Ammo (`self.AmmoAmount`))))
  (if (> _output_get (`self.MaxMagazineSize`))
    (set `self.AmmoAmount` (`self.MaxMagazineSize`))))

(fn `UserConstructionScript`)