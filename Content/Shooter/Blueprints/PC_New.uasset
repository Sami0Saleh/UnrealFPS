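; Player controller for the shooter that handles player input and creates the HUD.
; On BeginPlay it adds an Enhanced Input mapping context, then routes move, look, jump and crouch actions to player 0's pawn or character.
; Shoot and weapon switch are forwarded to the pawn as messages, leaving their implementation to the pawn.
; Each possession creates a new HUD widget and adds it to the viewport.
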(event `self.ReceiveBeginPlay`
  (`EnhancedInputSubsystemInterface.AddMappingContext` (pcsubsystem `EnhancedInputLocalPlayerSubsystem` self) "/Game/Shooter/Input/IMC_Override.IMC_Override" 0 (struct)))

(event `EnhancedInput|/Game/Shooter/Input/Actions/IA_NewShoot`
  (params (ActionValue :type Boolean) (ElapsedSeconds :type "Float (double-precision)") (TriggeredSeconds :type "Float (double-precision)") (InputAction :type "InputAction Object Reference" :default "/Game/Shooter/Input/Actions/IA_NewShoot.IA_NewShoot"))
  (:`Triggered`
    (message `/Game/Shooter/Blueprints/BPI_player.Attack` (`GameplayStatics.GetPlayerPawn` 0))))

(event `EnhancedInput|/Game/Shooter/Input/Actions/IA_NewMove`
  (params (ActionValue :type "Vector2D Structure") (ElapsedSeconds :type "Float (double-precision)") (TriggeredSeconds :type "Float (double-precision)") (InputAction :type "InputAction Object Reference" :default "/Game/Shooter/Input/Actions/IA_NewMove.IA_NewMove"))
  (bind _returnvalue (`GameplayStatics.GetPlayerPawn` 0))
  (bind (_x _y) (`KismetMathLibrary.BreakVector2D` ActionValue))
  (:`Triggered`
    (`Pawn.AddMovementInput` _returnvalue (`self.GetActorForwardVector` _returnvalue) _y false)
    (`Pawn.AddMovementInput` _returnvalue (`self.GetActorRightVector` _returnvalue) _x false)))

(event `EnhancedInput|/Game/Shooter/Input/Actions/IA_NewJump`
  (params (ActionValue :type Boolean) (ElapsedSeconds :type "Float (double-precision)") (TriggeredSeconds :type "Float (double-precision)") (InputAction :type "InputAction Object Reference" :default "/Game/Shooter/Input/Actions/IA_NewJump.IA_NewJump"))
  (:`Triggered`
    (`Character.Jump` (`GameplayStatics.GetPlayerCharacter` 0))))

(event `EnhancedInput|/Game/Shooter/Input/Actions/IA_NewLook`
  (params (ActionValue :type "Vector2D Structure") (ElapsedSeconds :type "Float (double-precision)") (TriggeredSeconds :type "Float (double-precision)") (InputAction :type "InputAction Object Reference" :default "/Game/Shooter/Input/Actions/IA_NewLook.IA_NewLook"))
  (bind (_x _y) (`KismetMathLibrary.BreakVector2D` ActionValue))
  (bind _returnvalue (`GameplayStatics.GetPlayerPawn` 0))
  (:`Triggered`
    (`Pawn.AddControllerYawInput` _returnvalue _x)
    (`Pawn.AddControllerPitchInput` _returnvalue (* _y -1.0))))

(event `EnhancedInput|/Game/Shooter/Input/Actions/IA_NewCrouch`
  (params (ActionValue :type Boolean) (ElapsedSeconds :type "Float (double-precision)") (TriggeredSeconds :type "Float (double-precision)") (InputAction :type "InputAction Object Reference" :default "/Game/Shooter/Input/Actions/IA_NewCrouch.IA_NewCrouch"))
  (bind _returnvalue (`GameplayStatics.GetPlayerCharacter` 0))
  (:`Started`
    (`Character.Crouch` _returnvalue))
  (:`Completed`
    (`Character.UnCrouch` _returnvalue)))

(event `EnhancedInput|/Game/Shooter/Input/Actions/IA_SwitchWeapon`
  (params (ActionValue :type Boolean) (ElapsedSeconds :type "Float (double-precision)") (TriggeredSeconds :type "Float (double-precision)") (InputAction :type "InputAction Object Reference" :default "/Game/Shooter/Input/Actions/IA_SwitchWeapon.IA_SwitchWeapon"))
  (:`Started`
    (message `/Game/Shooter/Blueprints/BPI_player.SwitchWeapon` (`GameplayStatics.GetPlayerPawn` 0))))

(event `self.ReceivePossess`
  (params (PossessedPawn :type "Pawn Object Reference"))
  (bind _returnvalue (`|CreateWidget` "/Game/Shooter/UI/UI_HUD.UI_HUD_C" self))
  (`UserWidget.AddToViewport` _returnvalue 0))

(fn `UserConstructionScript`)