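; BP_Bullet is a shooter projectile whose material and damage depend on its WeaponType, either Rifle or Mashinegun, set on BeginPlay.
; When its Sphere hits, it looks up a single BP_Guard with GetActorOfClass and tests whether the hit actor overlaps that guard, rather than being it.
; If so, it sends the guard TakeDamageMessage and calls OnHitOfBullet with the damage.
; The bullet destroys itself after any hit.
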(event `self.ReceiveBeginPlay`
  (switch `/Game/Shooter/Enums/E_WeaponType` (`self.WeaponType`)
    (:`NewEnumerator0`
      (`PrimitiveComponent.SetMaterial` (`self.Sphere`) 0 "/Game/FPWeapon/Mesh/Magazine/default_material.default_material")
      (set `self.Damage` 10))
    (:`NewEnumerator1`
      (`PrimitiveComponent.SetMaterial` (`self.Sphere`) 0 "/Game/FPWeapon/Materials/FirstPersonProjectileMaterial.FirstPersonProjectileMaterial")
      (set `self.Damage` 100))))

(event `self.Sphere.OnComponentHit`
  (params (HitComponent :type "PrimitiveComponent Object Reference") (OtherActor :type "Actor Object Reference") (OtherComp :type "PrimitiveComponent Object Reference") (NormalImpulse :type "Vector Structure") (Hit :type "HitResult Structure (by ref)"))
  (bind _damage (`self.Damage`))
  (bind _returnvalue (`GameplayStatics.GetActorOfClass` "/Game/Shooter/Blueprints/BP_Guard.BP_Guard_C"))
  (if (`self.IsOverlappingActor` OtherActor _returnvalue)
    (message `/Game/Shooter/Blueprints/BPI_Guard.TakeDamage` _returnvalue _damage)
    (`self.OnHitOfBullet` _damage)
    (`self.K2_DestroyActor`)
    (else
      (`self.K2_DestroyActor`))))

(fn `UserConstructionScript`)