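; Shooter guard AI that patrols between PointA and PointB, with health set by Normal or Heavy type and destruction at zero.
; DetectionRadius overlaps trigger a visibility multi-trace from HeadPivot.
; On a player hit, it turns toward the player, waits, then moves to the player's sampled location if still in range, otherwise resumes patrolling.
; A Patrol/Detection/Chase state switch exists but is disconnected, so State drives nothing.
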(event `self.ReceiveBeginPlay`
  (switch `/Game/Shooter/Enums/E_GuardType` (`self.Type`)
    (:`NewEnumerator0`
      (set `self.Health` 100))
    (:`NewEnumerator1`
      (set `self.Health` 200)))
  (`KismetSystemLibrary.Delay` 1.0 :!label _label)
  (bind _movementresult (`|AIMoveTo` self (0.0 0.0 0.0) (`self.PointA`) 100.0 true)
    (:`OnSuccess`
      (`KismetSystemLibrary.Delay` 1.0)
      (bind _movementresult_2 (`|AIMoveTo` self (0.0 0.0 0.0) (`self.PointB`) 100.0 true)
        (:`OnSuccess`
          (goto _label))
        (:`OnFail`
          (`KismetSystemLibrary.PrintString` (`|GetEnumeratorNameAsString` _movementresult_2)))))
    (:`OnFail`
      (`KismetSystemLibrary.PrintString` (`|GetEnumeratorNameAsString` _movementresult)))))

(event `self.ReceiveTick`
  (params (DeltaSeconds :type "Float (single-precision)")))

(event `/Game/Shooter/Blueprints/BPI_Guard.TakeDamage`
  (params (Damage :type Integer))
  (bind _output_get (set `self.Health` (- (`self.Health`) Damage)))
  (if (<= _output_get 0)
    (`self.K2_DestroyActor`)))

(event `self.DetectionRadius.OnComponentBeginOverlap`
  (params (OverlappedComponent :type "PrimitiveComponent Object Reference") (OtherActor :type "Actor Object Reference") (OtherComp :type "PrimitiveComponent Object Reference") (OtherBodyIndex :type Integer) (bFromSweep :type Boolean) (SweepResult :type "HitResult Structure (by ref)"))
  (bind _returnvalue (`SceneComponent.K2_GetComponentLocation` (`self.HeadPivot`)))
  (if (`self.IsOverlappingActor` OtherActor (`GameplayStatics.GetPlayerPawn` 0))
    (bind _outhits (`KismetSystemLibrary.LineTraceMulti` :`Start` _returnvalue :`End` (+ _returnvalue (`SceneComponent.K2_GetComponentLocation` (`self.DetectionRadius`))) :`TraceChannel` "TraceTypeQuery1" :`DrawDebugType` "ForDuration"))
    (for _array_element _outhits
      (if (== (`.HitActor` (`GameplayStatics.BreakHitResult` _array_element)) (`GameplayStatics.GetPlayerPawn` 0))
        (`self.RotateToPlayer`)
        (`KismetSystemLibrary.Delay` 3.0)
        (if (`PrimitiveComponent.IsOverlappingActor` (`self.DetectionRadius`) (`GameplayStatics.GetPlayerPawn` 0))
          (`|AIMoveTo` self (`self.K2_GetActorLocation` (`GameplayStatics.GetPlayerPawn` 0)) null 100.0
            (:`OnFail`
              (set `self.State` "NewEnumerator0")))
          (else
            (bind _movementresult (`|AIMoveTo` self (0.0 0.0 0.0) (`self.PointA`) 100.0 true :!label _label_2)
              (:`OnSuccess`
                (`KismetSystemLibrary.Delay` 1.0)
                (bind _movementresult_2 (`|AIMoveTo` self (0.0 0.0 0.0) (`self.PointB`) 100.0 true)
                  (:`OnSuccess`
                    (`KismetSystemLibrary.Delay` 1.0 :!label _label_3)
                    (goto _label_2))
                  (:`OnFail`
                    (`KismetSystemLibrary.PrintString` (`|GetEnumeratorNameAsString` _movementresult_2)))))
              (:`OnFail`
                (`KismetSystemLibrary.PrintString` (`|GetEnumeratorNameAsString` _movementresult))))))))
    (else
      (goto _label_3))))

(fn `RotateToPlayer`
  (`self.K2_SetActorRotation` (`KismetMathLibrary.FindLookAtRotation` (`self.K2_GetActorLocation`) (`self.K2_GetActorLocation` (`GameplayStatics.GetPlayerPawn` 0)))))

(fn `UserConstructionScript`)