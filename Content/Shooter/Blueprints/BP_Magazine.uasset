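; BP_Magazine is an ammo pickup for rifle or machinegun that holds a random amount of ammo.
; On BeginPlay, its type sets the material and ammo range, and the count feeds a hidden UI_Magazine widget.
; WidgetRadios overlap shows or hides that widget for BPI_player actors.
; PickupRadios overlap sends the ammo to Pawn_FPS, then destroys the magazine and updates the PC_New HUD if the pawn has a weapon and can add ammo.
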(event `self.ReceiveBeginPlay`
  ;[1 1 1] Set Random Amount For The Magazine
  (`SceneComponent.SetHiddenInGame` (`self.Amount`) true false)
  (switch `/Game/Shooter/Enums/E_WeaponType` (`self.CurrentMagazineType`)
    (:`NewEnumerator0`
      (`PrimitiveComponent.SetMaterial` (`self.StaticMesh`) 0 "/Game/ImportedAssets/FPWeapon/Mesh/Magazine/default_material.default_material")
      (bind _output_get (set `self.AmmoCount` (`KismetMathLibrary.RandomIntegerInRange` 10 20)))
      (bind _asui_magazine (cast `/Game/Shooter/UI/UI_Magazine` (`WidgetComponent.GetWidget` (`self.Amount`))))
      (set `/Game/Shooter/UI/UI_Magazine.Amount` _output_get _asui_magazine))
    (:`NewEnumerator1`
      (`PrimitiveComponent.SetMaterial` (`self.StaticMesh`) 0 "/Game/ImportedAssets/FPWeapon/Mesh/Magazine/New_material.New_material")
      (bind _output_get_2 (set `self.AmmoCount` (`KismetMathLibrary.RandomIntegerInRange` 5 10)))
      (bind _asui_magazine_2 (cast `/Game/Shooter/UI/UI_Magazine` (`WidgetComponent.GetWidget` (`self.Amount`))))
      (set `/Game/Shooter/UI/UI_Magazine.Amount` _output_get_2 _asui_magazine_2))))

(event `self.PickupRadios.OnComponentBeginOverlap`
  (params (OverlappedComponent :type "PrimitiveComponent Object Reference") (OtherActor :type "Actor Object Reference") (OtherComp :type "PrimitiveComponent Object Reference") (OtherBodyIndex :type Integer) (bFromSweep :type Boolean) (SweepResult :type "HitResult Structure (by ref)"))
  ;[1 1 1] Pickup The Magazine
  (bind _aspawn_fps (cast `/Game/Shooter/Blueprints/Pawn_FPS` OtherActor))
  (message `/Game/Shooter/Blueprints/BPI_player.AddAmmo` _aspawn_fps (`self.AmmoCount`) (`self.CurrentMagazineType`))
  (if (`/Game/Shooter/Blueprints/Pawn_FPS.HasWeapon` _aspawn_fps)
    (if (`/Game/Shooter/Blueprints/Pawn_FPS.CanAddAmmo` _aspawn_fps)
      (`self.K2_DestroyActor`)
      (bind _returnvalue (`GameplayStatics.GetActorOfClass` "/Game/Shooter/Blueprints/PC_New.PC_New_C"))
      (`/Game/Shooter/Blueprints/PC_New.UpdateHUD` _returnvalue))))

(event `self.WidgetRadios.OnComponentBeginOverlap`
  (params (OverlappedComponent :type "PrimitiveComponent Object Reference") (OtherActor :type "Actor Object Reference") (OtherComp :type "PrimitiveComponent Object Reference") (OtherBodyIndex :type Integer) (bFromSweep :type Boolean) (SweepResult :type "HitResult Structure (by ref)"))
  ;[1 1 1] Show magazine amount
  (if (`KismetSystemLibrary.DoesImplementInterface` OtherActor "/Game/Shooter/Blueprints/BPI_player.BPI_player_C")
    (`SceneComponent.SetHiddenInGame` (`self.Amount`) false false)))

(event `self.WidgetRadios.OnComponentEndOverlap`
  (params (OverlappedComponent :type "PrimitiveComponent Object Reference") (OtherActor :type "Actor Object Reference") (OtherComp :type "PrimitiveComponent Object Reference") (OtherBodyIndex :type Integer))
  ;[1 1 1] Hide magazine amount
  (if (`KismetSystemLibrary.DoesImplementInterface` OtherActor "/Game/Shooter/Blueprints/BPI_player.BPI_player_C")
    (`SceneComponent.SetHiddenInGame` (`self.Amount`) true false)))

(fn `UserConstructionScript`)