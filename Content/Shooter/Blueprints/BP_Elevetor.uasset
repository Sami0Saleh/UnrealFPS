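; Elevator actor that moves between two referenced target actors when a player enters its trigger box.
; A Box overlap with any actor implementing BPI_player plays a Timeline from the start.
; Each update feeds Alpha to ChangeLocationByAlpha, which lerps the elevator from TargetA's location to TargetB's without sweep.
; Re-entering the box restarts the Timeline, and no separate return logic exists.
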(event `self.ReceiveBeginPlay`)

(event `self.Box.OnComponentBeginOverlap`
  (params (OverlappedComponent :type "PrimitiveComponent Object Reference") (OtherActor :type "Actor Object Reference") (OtherComp :type "PrimitiveComponent Object Reference") (OtherBodyIndex :type Integer) (bFromSweep :type Boolean) (SweepResult :type "HitResult Structure (by ref)"))
  (if (`KismetSystemLibrary.DoesImplementInterface` OtherActor "/Game/Shooter/Blueprints/BPI_player.BPI_player_C")
    (bind (_direction _alpha) (`Timeline|Timeline` :!via `PlayFromStart`)
      (:`Update`
        (`self.ChangeLocationByAlpha` _alpha)))))

(fn `ChangeLocationByAlpha`
  (params (Alpha :type "Float (single-precision)"))
  (`self.K2_SetActorLocation` (`KismetMathLibrary.VLerp` (`self.K2_GetActorLocation` (`self.Target A`)) (`self.K2_GetActorLocation` (`self.Target B`)) Alpha)))

(fn `UserConstructionScript`)