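; GM_FPS is a Blueprint, apparently the shooter's game mode, that tracks how many guards are alive and shows it on the HUD.
; On BeginPlay it finds every BP_Guard and binds to its start and death dispatchers.
; Guard starts raise the max and current counts, creating the UI_HUD widget on the first call and updating it afterwards.
; Guard deaths lower the current count and refresh the HUD.
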(event `self.ReceiveBeginPlay`
  (bind _outactors (`GameplayStatics.GetAllActorsOfClass` "/Game/Shooter/Blueprints/BP_Guard.BP_Guard_C"))
  (for _array_element _outactors
    (add `/Game/Shooter/Blueprints/BP_Guard.OnGuardStart` _array_element (delegate `OnGuardStart_Event`))
    (add `/Game/Shooter/Blueprints/BP_Guard.OnDead` _array_element (delegate `OnGuardDead_Event`))))

(event `OnGuardDead_Event`
  ;[1 1 1] Bind to OnGuardDead & update the HUD
  (`/Engine/EditorBlueprintResources/StandardMacros.DecrementInt` (`self.GuardCount`)
    (:`  `
      (`/Game/Shooter/UI/UI_HUD.UpdateHUD` (`self.HUDRef`) (`self.MaxGuardCount`) (`self.GuardCount`)))))

(event `OnGuardStart_Event`
  ;[1 1 1] Bind to OnGuardStart & update the HUD
  (`/Engine/EditorBlueprintResources/StandardMacros.IncrementInt` (`self.MaxGuardCount`)
    (:`  `
      (`/Engine/EditorBlueprintResources/StandardMacros.IncrementInt` (`self.GuardCount`)
        (:`  `
          (if (`self.IsHUDCreated`)
            (`/Game/Shooter/UI/UI_HUD.UpdateHUD` (`self.HUDRef`) (`self.MaxGuardCount`) (`self.GuardCount`))
            (else
              (bind _returnvalue (`|CreateWidget` "/Game/Shooter/UI/UI_HUD.UI_HUD_C"))
              (bind _output_get (set `self.HUDRef` _returnvalue))
              (`/Game/Shooter/UI/UI_HUD.CreateHUD` _output_get (`self.MaxGuardCount`) (`self.GuardCount`))
              (`UserWidget.AddToViewport` _output_get 0)
              (set `self.IsHUDCreated` true))))))))

(fn `UserConstructionScript`)